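; Puzzle button actor whose cube mesh shows an off, on or complete state through material swaps.
; ReverseOn toggles the button and Off switches it off, both ignored once Done has marked it complete.
; The construction script applies the complete material to buttons flagged Rest, without setting the Complete flag.
; The Blueprint has no active events of its own, so state changes come only through these functions.
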(fn `done`
  (set `self.Complete?` true)
  (`PrimitiveComponent.SetMaterial` (`self.Cube`) 0 "/Game/Roles/Programmer/Sakith_BuildMasterExtraordinaire/Puzzels/Buttom_Puzzel/Button_Compleate.Button_Compleate"))

(fn `off`
  (if (not (`self.Complete?`))
    (if (== (`self.On?`) true)
      (set `self.On?` false)
      (`PrimitiveComponent.SetMaterial` (`self.Cube`) 0 "/Game/Roles/Programmer/Sakith_BuildMasterExtraordinaire/Puzzels/Buttom_Puzzel/Button_Off.Button_Off"))))

(fn `reverse on`
  (if (not (`self.Complete?`))
    (bind _output_get (set `self.On?` (not (`self.On?`))))
    (if _output_get
      (`PrimitiveComponent.SetMaterial` (`self.Cube`) 0 "/Game/Roles/Programmer/Sakith_BuildMasterExtraordinaire/Puzzels/Buttom_Puzzel/Button_On.Button_On")
      (else
        (`PrimitiveComponent.SetMaterial` (`self.Cube`) 0 "/Game/Roles/Programmer/Sakith_BuildMasterExtraordinaire/Puzzels/Buttom_Puzzel/Button_Off.Button_Off")))))

(fn `UserConstructionScript`
  (if (`self.rest`)
    (`PrimitiveComponent.SetMaterial` (`self.Cube`) 0 "/Game/Roles/Programmer/Sakith_BuildMasterExtraordinaire/Puzzels/Buttom_Puzzel/Button_Compleate.Button_Compleate")))