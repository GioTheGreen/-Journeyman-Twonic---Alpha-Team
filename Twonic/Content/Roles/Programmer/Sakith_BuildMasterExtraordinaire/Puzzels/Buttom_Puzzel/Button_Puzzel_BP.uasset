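; Lights Out style puzzle actor with a 3x3 grid of Button_BP child actors, each paired with a box trigger.
; Overlapping a box flips that button and its orthogonal neighbours through Inverse, without filtering which actor overlapped.
; After each flip, Check scans the button array built on BeginPlay and calls Done on every button once all are on.
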(event `self.ReceiveBeginPlay`
  ;[1 1 1] create array
  (set `self.Buttons` (`|MakeArray` (`self.Button_TL`) (`self.Button_TM`) (`self.Button_TR`) (`self.Button_ML`) (`self.Button_MM`) (`self.Button_MR`) (`self.Button_BL`) (`self.Button_BM`) (`self.Button_BR`))))

(event `self.Box_TL.OnComponentBeginOverlap`
  (params (OverlappedComponent :type "PrimitiveComponent Object Reference") (OtherActor :type "Actor Object Reference") (OtherComp :type "PrimitiveComponent Object Reference") (OtherBodyIndex :type Integer) (bFromSweep :type Boolean) (SweepResult :type "HitResult Structure (by ref)"))
  ;[1 1 1] not checking player yet
  (`self.Inverse` (`|MakeArray` (`self.Button_TM`) (`self.Button_TL`) (`self.Button_ML`))))

(event `self.Box_TM.OnComponentBeginOverlap`
  (params (OverlappedComponent :type "PrimitiveComponent Object Reference") (OtherActor :type "Actor Object Reference") (OtherComp :type "PrimitiveComponent Object Reference") (OtherBodyIndex :type Integer) (bFromSweep :type Boolean) (SweepResult :type "HitResult Structure (by ref)"))
  ;[1 1 1] not checking player yet
  (`self.Inverse` (`|MakeArray` (`self.Button_TL`) (`self.Button_TM`) (`self.Button_TR`) (`self.Button_MM`))))

(event `self.Box_TR.OnComponentBeginOverlap`
  (params (OverlappedComponent :type "PrimitiveComponent Object Reference") (OtherActor :type "Actor Object Reference") (OtherComp :type "PrimitiveComponent Object Reference") (OtherBodyIndex :type Integer) (bFromSweep :type Boolean) (SweepResult :type "HitResult Structure (by ref)"))
  ;[1 1 1] not checking player yet
  (`self.Inverse` (`|MakeArray` (`self.Button_TM`) (`self.Button_TR`) (`self.Button_MR`))))

(event `self.Box_ML.OnComponentBeginOverlap`
  (params (OverlappedComponent :type "PrimitiveComponent Object Reference") (OtherActor :type "Actor Object Reference") (OtherComp :type "PrimitiveComponent Object Reference") (OtherBodyIndex :type Integer) (bFromSweep :type Boolean) (SweepResult :type "HitResult Structure (by ref)"))
  ;[1 1 1] not checking player yet
  (`self.Inverse` (`|MakeArray` (`self.Button_TL`) (`self.Button_ML`) (`self.Button_MM`) (`self.Button_BL`))))

(event `self.Box_MM.OnComponentBeginOverlap`
  (params (OverlappedComponent :type "PrimitiveComponent Object Reference") (OtherActor :type "Actor Object Reference") (OtherComp :type "PrimitiveComponent Object Reference") (OtherBodyIndex :type Integer) (bFromSweep :type Boolean) (SweepResult :type "HitResult Structure (by ref)"))
  ;[1 1 1] not checking player yet
  (`self.Inverse` (`|MakeArray` (`self.Button_TM`) (`self.Button_ML`) (`self.Button_MM`) (`self.Button_MR`) (`self.Button_BM`))))

(event `self.Box_MR.OnComponentBeginOverlap`
  (params (OverlappedComponent :type "PrimitiveComponent Object Reference") (OtherActor :type "Actor Object Reference") (OtherComp :type "PrimitiveComponent Object Reference") (OtherBodyIndex :type Integer) (bFromSweep :type Boolean) (SweepResult :type "HitResult Structure (by ref)"))
  ;[1 1 1] not checking player yet
  (`self.Inverse` (`|MakeArray` (`self.Button_TR`) (`self.Button_MM`) (`self.Button_MR`) (`self.Button_BR`))))

(event `self.Box_BL.OnComponentBeginOverlap`
  (params (OverlappedComponent :type "PrimitiveComponent Object Reference") (OtherActor :type "Actor Object Reference") (OtherComp :type "PrimitiveComponent Object Reference") (OtherBodyIndex :type Integer) (bFromSweep :type Boolean) (SweepResult :type "HitResult Structure (by ref)"))
  ;[1 1 1] not checking player yet
  (`self.Inverse` (`|MakeArray` (`self.Button_ML`) (`self.Button_BL`) (`self.Button_BM`))))

(event `self.Box_BM.OnComponentBeginOverlap`
  (params (OverlappedComponent :type "PrimitiveComponent Object Reference") (OtherActor :type "Actor Object Reference") (OtherComp :type "PrimitiveComponent Object Reference") (OtherBodyIndex :type Integer) (bFromSweep :type Boolean) (SweepResult :type "HitResult Structure (by ref)"))
  ;[1 1 1] not checking player yet
  (`self.Inverse` (`|MakeArray` (`self.Button_MM`) (`self.Button_BL`) (`self.Button_BM`) (`self.Button_BR`))))

(event `self.Box_BR.OnComponentBeginOverlap`
  (params (OverlappedComponent :type "PrimitiveComponent Object Reference") (OtherActor :type "Actor Object Reference") (OtherComp :type "PrimitiveComponent Object Reference") (OtherBodyIndex :type Integer) (bFromSweep :type Boolean) (SweepResult :type "HitResult Structure (by ref)"))
  ;[1 1 1] not checking player yet
  (`self.Inverse` (`|MakeArray` (`self.Button_MR`) (`self.Button_BM`) (`self.Button_BR`))))

(fn `check`
  (set `self.Complete` true)
  (for _array_element (`self.Buttons`)
    (bind _asbutton_bp (cast `/Game/Roles/Programmer/Sakith_BuildMasterExtraordinaire/Puzzels/Buttom_Puzzel/Button_BP` (`ChildActorComponent.ChildActor` _array_element)))
    (if (not (`/Game/Roles/Programmer/Sakith_BuildMasterExtraordinaire/Puzzels/Buttom_Puzzel/Button_BP.On?` _asbutton_bp))
      (set `self.Complete` false)))
  (if (`self.Complete`)
    (for _array_element_2 (`self.Buttons`)
      (bind _asbutton_bp_2 (cast `/Game/Roles/Programmer/Sakith_BuildMasterExtraordinaire/Puzzels/Buttom_Puzzel/Button_BP` (`ChildActorComponent.ChildActor` _array_element_2)))
      (`/Game/Roles/Programmer/Sakith_BuildMasterExtraordinaire/Puzzels/Buttom_Puzzel/Button_BP.done` _asbutton_bp_2))))

(fn `Inverse`
  (params (Array :type "Array of ChildActorComponent Object Reference"))
  (for _array_element Array
    (bind _asbutton_bp (cast `/Game/Roles/Programmer/Sakith_BuildMasterExtraordinaire/Puzzels/Buttom_Puzzel/Button_BP` (`ChildActorComponent.ChildActor` _array_element)))
    (`/Game/Roles/Programmer/Sakith_BuildMasterExtraordinaire/Puzzels/Buttom_Puzzel/Button_BP.reverse on` _asbutton_bp))
  (`self.check`))

(fn `UserConstructionScript`)