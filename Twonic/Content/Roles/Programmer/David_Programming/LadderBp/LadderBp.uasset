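; Ladder actor that lets the player's Twonic_Player_BP climb, with a widget shown during overlap.
; On box overlap, if the Climb input was already pressed, it orients player pawn 0 to the mesh transform cached at BeginPlay and enables climbing.
; Ending overlap hides the widget, clears the press flag and disables climbing.
; The flag is only checked on overlap begin, and the overlapping actor is not filtered.
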(event `self.Box.OnComponentBeginOverlap`
  (params (OverlappedComponent :type "PrimitiveComponent Object Reference") (OtherActor :type "Actor Object Reference") (OtherComp :type "PrimitiveComponent Object Reference") (OtherBodyIndex :type Integer) (bFromSweep :type Boolean) (SweepResult :type "HitResult Structure (by ref)"))
  ;[0.4464 1 0.3181] Ladder
  (`|ExecutionSequence`
    (:`then_0`
      (`SceneComponent.SetVisibility` (`self.Widget`) true false))
    (:`then_1`
      (if (`self.Button Pressed`)
        (bind _astwonic_player_bp (cast `/Game/Roles/Designer/Owen/Bps/Twonic_Player_BP` (`GameplayStatics.GetPlayerPawn` 0)))
        (`/Game/Roles/Designer/Owen/Bps/Twonic_Player_BP.OrientPlayer` _astwonic_player_bp (`self.Position`))
        (`/Game/Roles/Designer/Owen/Bps/Twonic_Player_BP.Toggle Climbing` _astwonic_player_bp true)))))

(event `InputAction|Climb`
  (params (Key :type "Key Structure"))
  ;[0.4464 1 0.3181] Ladder
  (:`Pressed`
    (set `self.Button Pressed` true)))

(event `self.Box.OnComponentEndOverlap`
  (params (OverlappedComponent :type "PrimitiveComponent Object Reference") (OtherActor :type "Actor Object Reference") (OtherComp :type "PrimitiveComponent Object Reference") (OtherBodyIndex :type Integer))
  ;[0.4464 1 0.3181] Ladder
  (`|ExecutionSequence`
    (:`then_0`
      (`SceneComponent.SetVisibility` (`self.Widget`) false false))
    (:`then_1`
      (set `self.Button Pressed` false)
      (bind _astwonic_player_bp (cast `/Game/Roles/Designer/Owen/Bps/Twonic_Player_BP` (`GameplayStatics.GetPlayerPawn` 0)))
      (`/Game/Roles/Designer/Owen/Bps/Twonic_Player_BP.Toggle Climbing` _astwonic_player_bp false))))

(event `self.ReceiveBeginPlay`
  ;[0.4464 1 0.3181] Ladder
  (set `self.Position` (`SceneComponent.K2_GetComponentToWorld` (`self.StaticMesh`))))

(fn `UserConstructionScript`)