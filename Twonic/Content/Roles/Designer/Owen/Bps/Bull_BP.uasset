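; Bull enemy character with health, hit reactions, death, and player sighting for its AI.
; Damage passes through a DoOnce gate that resets only after the hit-react montage's duration, so hits during the reaction are ignored.
; At zero health it plays the death montage and destroys its capsule component, leaving the gate closed.
; PawnSensing sets the "Has Seen Player?" blackboard key on spotting Twonic_Player_BP; nothing here clears it.
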(event `self.ReceiveBeginPlay`
  (bind _output_get (set `self.Health` 100.0))
  (bind _output_get_2 (set `self.Death` (<= _output_get 0.0)))
  (if _output_get_2
    (`self.PlayAnimMontage` "/Game/Roles/Designer/Owen/Anims/Death_Montage.Death_Montage")))

(event `self.ReceiveAnyDamage`
  (params (Damage :type "Float (single-precision)") (DamageType :type "DamageType Object Reference") (InstigatedBy :type "Controller Object Reference") (DamageCauser :type "Actor Object Reference"))
  (`/Engine/EditorBlueprintResources/StandardMacros.DoOnce` false :!label _label
    (:`Completed`
      (bind _output_get (set `self.Health` (- (`self.Health`) Damage)))
      (if (<= _output_get 0.0)
        (`self.PlayAnimMontage` "/Game/Roles/Designer/Owen/Anims/Death_Montage.Death_Montage")
        (`ActorComponent.K2_DestroyComponent` (`self.CapsuleComponent`))
        (else
          (bind _returnvalue (`self.PlayAnimMontage` "/Game/Roles/Designer/Owen/Anims/HitReact_Montage.HitReact_Montage"))
          (`KismetSystemLibrary.Delay` _returnvalue)
          (goto _label :!via `Reset`))))))

(event `self.PawnSensing.OnSeePawn`
  (params (Pawn :type "Pawn Object Reference"))
  (cast `/Game/Roles/Designer/Owen/Bps/Twonic_Player_BP` Pawn)
  (`BlackboardComponent.SetValueAsBool` (`AIBlueprintHelperLibrary.GetBlackboard` (`AIBlueprintHelperLibrary.GetAIController` self)) "Has Seen Player?" true))

(fn `UserConstructionScript`)