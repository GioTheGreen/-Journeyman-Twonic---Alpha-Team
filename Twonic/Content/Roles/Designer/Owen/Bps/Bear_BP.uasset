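; Bear enemy character that flags "Has Seen Player?" on its AI blackboard when pawn sensing spots the player.
; Damage updates a widget health bar, shown while the player overlaps a trigger, and is ignored until the block montage ends.
; Lethal damage plays death animation, roar and blood before destroying it; sling rock overlaps subtract health without a death check.
; Construction enables custom depth stencil on the mesh.
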(event `self.ReceiveBeginPlay`
  (bind _astwonic_player_bp (cast `/Game/Roles/Designer/Owen/Bps/Twonic_Player_BP` (`GameplayStatics.GetPlayerCharacter` 0)))
  (set `self.As Twonic Player BP` _astwonic_player_bp)
  (bind _asenemy_health_bar (cast `/Game/Roles/Designer/Owen/AI/Enemy_HealthBar` (`WidgetComponent.GetUserWidgetObject` (`self.Widget`))))
  (set `self.As Enemy Health Bar` _asenemy_health_bar)
  (set `self.Health` 100.0))

(event `self.ReceiveAnyDamage`
  (params (Damage :type "Float (single-precision)") (DamageType :type "DamageType Object Reference") (InstigatedBy :type "Controller Object Reference") (DamageCauser :type "Actor Object Reference"))
  (`/Engine/EditorBlueprintResources/StandardMacros.DoOnce` false :!label _label
    (:`Completed`
      (bind _output_get (set `self.Health` (- (`self.Health`) Damage)))
      (bind _output_get_2 (set `/Game/Roles/Designer/Owen/AI/Enemy_HealthBar.Health` _output_get (`self.As Enemy Health Bar`)))
      (if (<= _output_get_2 0.0)
        (set `self.Death` true)
        (`CharacterMovementComponent.DisableMovement` (`self.CharacterMovement`))
        (`self.PlayAnimMontage` "/Game/Roles/Designer/Owen/Anims/SmallBear/main_enemy_death_Montage.main_enemy_death_Montage")
        (`GameplayStatics.PlaySoundAtLocation` "/Game/Roles/Designer/Michael/SFX/Enemies/Bear/BearRoar.BearRoar" (`self.K2_GetActorLocation`) (struct) 1.0 1.0 0.0 null null null)
        (`KismetSystemLibrary.Delay` 3.0)
        (`GameplayStatics.SpawnEmitterAtLocation` "/Game/Roles/Designer/Lewis/Effects/ParticleSystems/PS_Impact_Blood.PS_Impact_Blood" (`SceneComponent.GetSocketLocation` (`self.Mesh`) "BleedSocket"))
        (`KismetSystemLibrary.Delay` 0.6)
        (`self.K2_DestroyActor`)
        (else
          (bind _returnvalue (`self.PlayAnimMontage` "/Game/Roles/Designer/Owen/Anims/SmallBear/main_enemy_block_Montage.main_enemy_block_Montage"))
          (`GameplayStatics.PlaySoundAtLocation` "/Game/Roles/Designer/Michael/SFX/Enemies/Bear/Bear_Grunt.Bear_Grunt" (`self.K2_GetActorLocation`) (struct) 1.0 1.0 0.0 null null null)
          (`KismetSystemLibrary.Delay` _returnvalue)
          (goto _label :!via `Reset`))))))

(event `self.PawnSensing.OnSeePawn`
  (params (Pawn :type "Pawn Object Reference"))
  (cast `/Game/Roles/Designer/Owen/Bps/Twonic_Player_BP` Pawn)
  (`BlackboardComponent.SetValueAsBool` (`AIBlueprintHelperLibrary.GetBlackboard` (`AIBlueprintHelperLibrary.GetAIController` self)) "Has Seen Player?" true))

(event `self.CapsuleComponent.OnComponentBeginOverlap`
  (params (OverlappedComponent :type "PrimitiveComponent Object Reference") (OtherActor :type "Actor Object Reference") (OtherComp :type "PrimitiveComponent Object Reference") (OtherBodyIndex :type Integer) (bFromSweep :type Boolean) (SweepResult :type "HitResult Structure (by ref)"))
  (cast `/Game/Roles/Designer/Owen/Bps/Sling_Rock` OtherActor)
  (bind _output_get (set `self.Health` (- (`self.Health`) 10.0)))
  (set `/Game/Roles/Designer/Owen/AI/Enemy_HealthBar.Health` _output_get (`self.As Enemy Health Bar`)))

(event `self.Hp bar spawner.OnComponentBeginOverlap`
  (params (OverlappedComponent :type "PrimitiveComponent Object Reference") (OtherActor :type "Actor Object Reference") (OtherComp :type "PrimitiveComponent Object Reference") (OtherBodyIndex :type Integer) (bFromSweep :type Boolean) (SweepResult :type "HitResult Structure (by ref)"))
  (cast `/Game/Roles/Designer/Owen/Bps/Twonic_Player_BP` OtherActor)
  (`SceneComponent.SetVisibility` (`self.Widget`) true false))

(event `self.Hp bar spawner.OnComponentEndOverlap`
  (params (OverlappedComponent :type "PrimitiveComponent Object Reference") (OtherActor :type "Actor Object Reference") (OtherComp :type "PrimitiveComponent Object Reference") (OtherBodyIndex :type Integer))
  (cast `/Game/Roles/Designer/Owen/Bps/Twonic_Player_BP` OtherActor)
  (`SceneComponent.SetVisibility` (`self.Widget`) false false))

(fn `UserConstructionScript`
  (`PrimitiveComponent.SetRenderCustomDepth` (`self.Mesh`) true)
  (`PrimitiveComponent.SetCustomDepthStencilValue` (`self.Mesh`) 2))