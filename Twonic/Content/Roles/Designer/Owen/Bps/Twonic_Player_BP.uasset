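; Twonic_Player_BP is a player character Blueprint that implements a stamina-costed dodge roll.
; The RollAnimation graph blocks further rolls, flags stamina use and rolling, deducts stamina, plays a dodge sound and triggers the DodgeRoll montage.
; It temporarily boosts walk speed for the roll, then a timed delay restores normal speed and clears the rolling flag.
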(fn `UserConstructionScript`)