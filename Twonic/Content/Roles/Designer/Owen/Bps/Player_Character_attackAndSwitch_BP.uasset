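; Player character with movement, jump, timeline-driven crouch and sprint, mouse-wheel weapon switching and a sword attack.
; Switching wraps through an inventory of mesh components, showing only the current one and snapping it to the sword's socket.
; Right-click plays the slash montage; separate trigger events toggle a looping timer that line-traces between blade sockets to apply damage.
; Hard landings ragdoll the character and load ThirdPersonExampleMap after a delay.
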(event `self.ReceiveBeginPlay`
  (bind _output_get (set `self.Weapon Inventory` (`|MakeArray` (`self.Sword Skeletal Mesh`) (`self.Weapon 2`) (`self.Weapon 3`) null)))
  (`self.Equip Weapon` _output_get))

(event `InputAxisKey|MouseWheelAxis`
  (params (AxisValue :type "Float (single-precision)"))
  (bind _returnvalue (+ (`KismetMathLibrary.FTrunc` AxisValue) (`self.Current Weapon`)))
  (if (`KismetArrayLibrary.Array_IsValidIndex` (`self.Weapon Inventory`) _returnvalue)
    (set `self.Current Weapon` _returnvalue)
    (`self.Equip Weapon` (`self.Weapon Inventory`))
    (elif (< _returnvalue 0)
      (set `self.Current Weapon` (`KismetArrayLibrary.Array_LastIndex` (`self.Weapon Inventory`)))
      (`self.Equip Weapon` (`self.Weapon Inventory`))
      (else
        (set `self.Current Weapon` 0)
        (`self.Equip Weapon` (`self.Weapon Inventory`))))))

(event `InputAxis|Forwards and Backwards Movement`
  (params (AxisValue :type "Float (single-precision)"))
  ;[1 1 1] Movment
  (`self.AddMovementInput` (`KismetMathLibrary.GetForwardVector` (`self.GetControlRotation`)) AxisValue))

(event `InputAxis|Left and Right Movement`
  (params (AxisValue :type "Float (single-precision)"))
  ;[1 1 1] Movment
  (`self.AddMovementInput` (`KismetMathLibrary.GetRightVector` (`self.GetControlRotation`)) AxisValue))

(event `InputAction|Jump`
  (params (Key :type "Key Structure"))
  ;[1 1 1] Movment
  (:`Pressed`
    (`self.Jump`)))

(event `InputAction|Crouch`
  (params (Key :type "Key Structure"))
  (bind _charactermovement (`self.CharacterMovement`))
  ;[1 1 1] Movment
  (:`Pressed`
    (set `CharacterMovementComponent.MaxWalkSpeed` 50.0 _charactermovement)
    (bind (_direction _crouch) (`Timeline|CrouchTimeLine` :!label _label)
      (:`Update`
        (`CapsuleComponent.SetCapsuleHalfHeight` (`self.CapsuleComponent`) (`KismetMathLibrary.Lerp` 90.0 50.0 _crouch) true))))
  (:`Released`
    (set `CharacterMovementComponent.MaxWalkSpeed` 400.0 _charactermovement)
    (goto _label :!via `Reverse`)))

(event `InputAction|Sprint`
  (params (Key :type "Key Structure"))
  (bind _charactermovement (`self.CharacterMovement`))
  ;[1 1 1] Movment
  (:`Pressed`
    (set `CharacterMovementComponent.MaxWalkSpeed` 600.0 _charactermovement)
    (bind (_direction _sprint) (`Timeline|SprintTimeline` :!label _label_2)
      (:`Update`
        (set `CharacterMovementComponent.MaxWalkSpeed` (`KismetMathLibrary.Lerp` (`self.Walk Speed`) (`self.Sprint Speed`) _sprint) (`self.CharacterMovement`)))))
  (:`Released`
    (set `CharacterMovementComponent.MaxWalkSpeed` 400.0 _charactermovement)
    (goto _label_2 :!via `Reverse`)))

(event `Key|RightMouseButton`
  (params (Key :type "Key Structure"))
  (:`Pressed`
    (`/Engine/EditorBlueprintResources/StandardMacros.DoOnce` false :!label _label_3
      (:`Completed`
        (bind _returnvalue (`self.PlayAnimMontage` "/Game/Roles/Designer/Owen/Anims/SwordSlash_Montage.SwordSlash_Montage"))
        (`KismetSystemLibrary.Delay` _returnvalue)
        (goto _label_3 :!via `Reset`)))))

(event `TriggerSword`
  (bind _returnvalue (`KismetSystemLibrary.K2_SetTimerDelegate` (delegate `SwordLineTrace`) 0.01 true))
  (set `self.TriggerSwordEvent` _returnvalue))

(event `SwordLineTrace`
  (bind _sword_skeletal_mesh (`self.Sword Skeletal Mesh`))
  (bind _outhit (`KismetSystemLibrary.LineTraceSingle` :`Start` (`SceneComponent.GetSocketLocation` _sword_skeletal_mesh "Start") :`End` (`SceneComponent.GetSocketLocation` _sword_skeletal_mesh "End") :`TraceChannel` "TraceTypeQuery2" :`DrawDebugType` "ForDuration"))
  (`GameplayStatics.ApplyDamage` (`.HitActor` (`GameplayStatics.BreakHitResult` _outhit)) 25.0))

(event `StopTriggerSword`
  (`KismetSystemLibrary.K2_ClearAndInvalidateTimerHandle` (`self.TriggerSwordEvent`)))

(event `self.OnLanded`
  (params (Hit :type "HitResult Structure (by ref)"))
  (bind (_returnvalue_x _returnvalue_y _returnvalue_z) (`KismetMathLibrary.BreakVector` (`self.GetVelocity`)))
  (bind _mesh (`self.Mesh`))
  (if (> (`KismetMathLibrary.Abs` _returnvalue_z) 700.0)
    (`KismetSystemLibrary.PrintString` "Ankles broken")
    (`PrimitiveComponent.SetSimulatePhysics` _mesh true)
    (`PrimitiveComponent.AddImpulse` _mesh (0.0 0.0 5000.0) "None" false)
    (`CharacterMovementComponent.DisableMovement` (`self.CharacterMovement`))
    (`KismetSystemLibrary.Delay` 5.0)
    (`GameplayStatics.OpenLevel` "ThirdPersonExampleMap")))

(fn `Equip Weapon`
  (params (Array :type "Array of SkeletalMeshComponent Object Reference"))
  (bind _output (`|GetArrayItem` Array (`self.Current Weapon`)))
  (for _array_element Array
    (`SceneComponent.SetVisibility` _array_element false false))
  (`SceneComponent.SetVisibility` _output true false)
  (`SceneComponent.K2_AttachToComponent` _output (`self.Sword Skeletal Mesh`) (`SceneComponent.GetAttachSocketName` (`self.Sword Skeletal Mesh`)) "SnapToTarget" "SnapToTarget" "SnapToTarget" true))

(fn `UserConstructionScript`
  (`SceneComponent.K2_SetWorldRotation` (`self.CameraBoom`) (struct :`Pitch` -10.0 :`Yaw` 45.0) false false))