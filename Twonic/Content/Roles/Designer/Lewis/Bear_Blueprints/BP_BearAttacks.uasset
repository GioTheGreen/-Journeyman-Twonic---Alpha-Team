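; BP_BearAttacks drives a bear enemy's slam, roar and swipe attacks, each started when the player overlaps its trigger.
; Slam spawns a shockwave and hitbox after a wind-up, while roar drops a timed series of rocks at random points in a nearby box.
; Swipe spawns immediately, angled off the Arrow's yaw.
; A DoOnce per attack blocks retriggering until its sequence or cooldown ends, with debug prints marking slam and roar phases.
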(event `self.SlamTrigger.OnComponentBeginOverlap`
  (params (OverlappedComponent :type "PrimitiveComponent Object Reference") (OtherActor :type "Actor Object Reference") (OtherComp :type "PrimitiveComponent Object Reference") (OtherBodyIndex :type Integer) (bFromSweep :type Boolean) (SweepResult :type "HitResult Structure (by ref)"))
  (bind _returnvalue (`KismetMathLibrary.Conv_VectorToTransform` (`self.K2_GetActorLocation`)))
  (cast `/Game/Roles/Designer/Owen/Bps/Twonic_Player_BP` OtherActor)
  (`/Engine/EditorBlueprintResources/StandardMacros.DoOnce` false :!label _label
    (:`Completed`
      (`KismetSystemLibrary.PrintString` "Bear raises arms" true true (struct :`R` 1.0 :`A` 1.0))
      (`KismetSystemLibrary.Delay` 1.0)
      (`|SpawnActorFromClass` "/Game/Roles/Designer/Lewis/Bear_Blueprints/BP_SlamShockwave.BP_SlamShockwave_C" _returnvalue "Undefined" "OverrideRootScale" null null)
      (`|SpawnActorFromClass` "/Game/Roles/Designer/Lewis/Bear_Blueprints/BP_SlamHitbox.BP_SlamHitbox_C" _returnvalue "Undefined" "OverrideRootScale" null null)
      (`KismetSystemLibrary.PrintString` "Bear slams down" true true (struct :`R` 1.0 :`A` 1.0))
      (goto _label :!via `Reset`))))

(event `self.RoarTrigger.OnComponentBeginOverlap`
  (params (OverlappedComponent :type "PrimitiveComponent Object Reference") (OtherActor :type "Actor Object Reference") (OtherComp :type "PrimitiveComponent Object Reference") (OtherBodyIndex :type Integer) (bFromSweep :type Boolean) (SweepResult :type "HitResult Structure (by ref)"))
  (cast `/Game/Roles/Designer/Owen/Bps/Twonic_Player_BP` OtherActor)
  (`/Engine/EditorBlueprintResources/StandardMacros.DoOnce` false :!label _label_2
    (:`Completed`
      (`KismetSystemLibrary.PrintString` "Roar Starts" true true (struct :`R` 1.0 :`A` 1.0))
      (`KismetSystemLibrary.Delay` 0.5)
      (`/Game/Roles/Designer/Lewis/Bear_Blueprints/BP_MacroLibrary.For_Loop_with_Delay` 0 4 1.0
        (:`Loop Body`
          (`|SpawnActorFromClass` "/Game/Roles/Designer/Lewis/Bear_Blueprints/BP_FallenRock.BP_FallenRock_C" (`KismetMathLibrary.Conv_VectorToTransform` (`KismetMathLibrary.RandomPointInBoundingBox` (- (`self.K2_GetActorLocation`) (-150.0 -150.0 0.0)) (300.0 300.0 0.0))) "Undefined" "OverrideRootScale" null null)
          (`KismetSystemLibrary.PrintString` "Rock Falls" true true (struct :`R` 1.0 :`A` 1.0)))
        (:`Completed`
          (`KismetSystemLibrary.PrintString` "Roar Ends" true true (struct :`R` 1.0 :`A` 1.0))
          (goto _label_2 :!via `Reset`))))))

(event `self.SwipeTrigger.OnComponentBeginOverlap`
  (params (OverlappedComponent :type "PrimitiveComponent Object Reference") (OtherActor :type "Actor Object Reference") (OtherComp :type "PrimitiveComponent Object Reference") (OtherBodyIndex :type Integer) (bFromSweep :type Boolean) (SweepResult :type "HitResult Structure (by ref)"))
  (bind (_returnvalue_roll _returnvalue_pitch _returnvalue_yaw) (`KismetMathLibrary.BreakRotator` (`SceneComponent.K2_GetComponentRotation` (`self.Arrow`))))
  (cast `/Game/Roles/Designer/Owen/Bps/Twonic_Player_BP` OtherActor)
  (`/Engine/EditorBlueprintResources/StandardMacros.DoOnce` false :!label _label_3
    (:`Completed`
      (`|SpawnActorFromClass` "/Game/Roles/Designer/Lewis/Bear_Blueprints/BP_BearSwipe.BP_BearSwipe_C" (`KismetMathLibrary.MakeTransform` (`self.K2_GetActorLocation`) (`KismetMathLibrary.MakeRotator` 0.0 0.0 (+ _returnvalue_yaw 45.0))) "Undefined" "OverrideRootScale" null null)
      (`KismetSystemLibrary.Delay` 3.5)
      (goto _label_3 :!via `Reset`))))

(fn `UserConstructionScript`)