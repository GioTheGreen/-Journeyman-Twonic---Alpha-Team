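; BP_BearSwipe is a bear swipe attack actor that sweeps back and forth in yaw, then destroys itself.
; On BeginPlay it records start and end yaw 90 degrees apart, then chains three timelines with short delays to rotate forward, back and forward again.
; Its Cube overlap only prints a hit message for the Twonic player, and destroys any BP_FallenRock it touches.
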(event `self.Cube.OnComponentBeginOverlap`
  (params (OverlappedComponent :type "PrimitiveComponent Object Reference") (OtherActor :type "Actor Object Reference") (OtherComp :type "PrimitiveComponent Object Reference") (OtherBodyIndex :type Integer) (bFromSweep :type Boolean) (SweepResult :type "HitResult Structure (by ref)"))
  (`|ExecutionSequence`
    (:`then_0`
      (cast `/Game/Roles/Designer/Owen/Bps/Twonic_Player_BP` OtherActor)
      (`KismetSystemLibrary.PrintString` "OW (Swipe)" true true (struct :`R` 1.0 :`A` 1.0)))
    (:`then_1`
      (bind _asbp_fallen_rock (cast `/Game/Roles/Designer/Lewis/Bear_Blueprints/BP_FallenRock` OtherActor))
      (`self.K2_DestroyActor` _asbp_fallen_rock))))

(event `self.ReceiveBeginPlay`
  (bind (_returnvalue_roll _returnvalue_pitch _returnvalue_yaw) (`KismetMathLibrary.BreakRotator` (`SceneComponent.K2_GetComponentRotation` (`self.DefaultSceneRoot`))))
  (set `self.Rotation Start` _returnvalue_yaw)
  (set `self.Rotation End` (+ _returnvalue_yaw 90.0))
  (`KismetSystemLibrary.Delay` 0.5)
  (bind (_direction _z__yaw_) (`Timeline|Swipe_1` :!via `PlayFromStart`)
    (:`Update`
      (`self.K2_SetActorRotation` (`KismetMathLibrary.MakeRotator` 0.0 0.0 (+ (`self.Rotation Start`) _z__yaw_))))
    (:`Finished`
      (`KismetSystemLibrary.Delay` 0.5)
      (bind (_direction_2 _z__yaw__2) (`Timeline|Swipe_2` :!via `PlayFromStart`)
        (:`Update`
          (`self.K2_SetActorRotation` (`KismetMathLibrary.MakeRotator` 0.0 0.0 (- (`self.Rotation End`) _z__yaw__2))))
        (:`Finished`
          (`KismetSystemLibrary.Delay` 0.5)
          (bind (_direction_3 _z__yaw__3) (`Timeline|Swipe_3` :!via `PlayFromStart`)
            (:`Update`
              (`self.K2_SetActorRotation` (`KismetMathLibrary.MakeRotator` 0.0 0.0 (+ (`self.Rotation Start`) _z__yaw__3))))
            (:`Finished`
              (`KismetSystemLibrary.Delay` 0.5)
              (`self.K2_DestroyActor`))))))))

(fn `UserConstructionScript`)