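; BP_SlamShockwave is a short-lived expanding shockwave actor, likely for the Bear's slam attack.
; On BeginPlay the Scaling timeline adds its XYScale to the Cylinder's current X and Y world scale each update, so growth accumulates per tick, then the actor destroys itself.
; Cylinder overlaps destroy any BP_FallenRock, while hits on Twonic_Player_BP only print a debug message, with no damage applied.
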(event `self.Cylinder.OnComponentBeginOverlap`
  (params (OverlappedComponent :type "PrimitiveComponent Object Reference") (OtherActor :type "Actor Object Reference") (OtherComp :type "PrimitiveComponent Object Reference") (OtherBodyIndex :type Integer) (bFromSweep :type Boolean) (SweepResult :type "HitResult Structure (by ref)"))
  (`|ExecutionSequence`
    (:`then_0`
      (cast `/Game/Roles/Designer/Owen/Bps/Twonic_Player_BP` OtherActor)
      (`KismetSystemLibrary.PrintString` "OW (Shockwave)" true true (struct :`R` 1.0 :`A` 1.0)))
    (:`then_1`
      (bind _asbp_fallen_rock (cast `/Game/Roles/Designer/Lewis/Bear_Blueprints/BP_FallenRock` OtherActor))
      (`self.K2_DestroyActor` _asbp_fallen_rock))))

(event `self.ReceiveBeginPlay`
  (bind (_returnvalue_x _returnvalue_y _returnvalue_z) (`KismetMathLibrary.BreakVector` (`SceneComponent.K2_GetComponentScale` (`self.Cylinder`))))
  (bind (_direction _x_y_scale) (`Timeline|Scaling`)
    (:`Update`
      (`SceneComponent.SetWorldScale3D` (`self.Cylinder`) (`KismetMathLibrary.MakeVector` (+ _x_y_scale _returnvalue_x) (+ _x_y_scale _returnvalue_y) _returnvalue_z)))
    (:`Finished`
      (`self.K2_DestroyActor`))))

(fn `UserConstructionScript`)