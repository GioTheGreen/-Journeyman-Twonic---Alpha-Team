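; Trigger-zone actor in a designer effects folder that spawns and clears heal, stamina and mana aura actors for the player.
; Overlapping the Heal, Stamina or Mana trigger spawns that aura at the player mesh's location and sets its active flag.
; The Clear trigger destroys each flagged aura and resets its flag.
; Spawning ignores the flags, so re-entering a trigger adds another aura.
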(event `self.HealTrigger.OnComponentBeginOverlap`
  (params (OverlappedComponent :type "PrimitiveComponent Object Reference") (OtherActor :type "Actor Object Reference") (OtherComp :type "PrimitiveComponent Object Reference") (OtherBodyIndex :type Integer) (bFromSweep :type Boolean) (SweepResult :type "HitResult Structure (by ref)"))
  (bind _astwonic_player_bp (cast `/Game/Roles/Designer/Owen/Bps/Twonic_Player_BP` OtherActor))
  (bind _returnvalue (`|SpawnActorFromClass` "/Game/Roles/Designer/Lewis/Effects/BP_Heal_Aura.BP_Heal_Aura_C" (`KismetMathLibrary.Conv_VectorToTransform` (`SceneComponent.K2_GetComponentLocation` (`Character.Mesh` _astwonic_player_bp))) "Undefined" "OverrideRootScale" null null))
  (set `self.HealOn` true))

(event `self.ClearTrigger.OnComponentBeginOverlap`
  (params (OverlappedComponent :type "PrimitiveComponent Object Reference") (OtherActor :type "Actor Object Reference") (OtherComp :type "PrimitiveComponent Object Reference") (OtherBodyIndex :type Integer) (bFromSweep :type Boolean) (SweepResult :type "HitResult Structure (by ref)"))
  (cast `/Game/Roles/Designer/Owen/Bps/Twonic_Player_BP` OtherActor)
  (`|ExecutionSequence`
    (:`then_0`
      (if (`self.HealOn`)
        (`self.K2_DestroyActor` (stale `self.HealTrigger.OnComponentBeginOverlap` _returnvalue))
        (set `self.HealOn` false)))
    (:`then_1`
      (if (`self.StaminaOn`)
        (`self.K2_DestroyActor` (stale `self.StaminaTrigger.OnComponentBeginOverlap` _returnvalue))
        (set `self.StaminaOn` false)))
    (:`then_2`
      (if (`self.ManaOn`)
        (`self.K2_DestroyActor` (stale `self.ManaTrigger.OnComponentBeginOverlap` _returnvalue))
        (set `self.ManaOn` false)))))

(event `self.StaminaTrigger.OnComponentBeginOverlap`
  (params (OverlappedComponent :type "PrimitiveComponent Object Reference") (OtherActor :type "Actor Object Reference") (OtherComp :type "PrimitiveComponent Object Reference") (OtherBodyIndex :type Integer) (bFromSweep :type Boolean) (SweepResult :type "HitResult Structure (by ref)"))
  (bind _astwonic_player_bp (cast `/Game/Roles/Designer/Owen/Bps/Twonic_Player_BP` OtherActor))
  (bind _returnvalue (`|SpawnActorFromClass` "/Game/Roles/Designer/Lewis/Effects/BP_Stamina_Aura.BP_Stamina_Aura_C" (`KismetMathLibrary.Conv_VectorToTransform` (`SceneComponent.K2_GetComponentLocation` (`Character.Mesh` _astwonic_player_bp))) "Undefined" "OverrideRootScale" null null))
  (set `self.StaminaOn` true))

(event `self.ManaTrigger.OnComponentBeginOverlap`
  (params (OverlappedComponent :type "PrimitiveComponent Object Reference") (OtherActor :type "Actor Object Reference") (OtherComp :type "PrimitiveComponent Object Reference") (OtherBodyIndex :type Integer) (bFromSweep :type Boolean) (SweepResult :type "HitResult Structure (by ref)"))
  (bind _astwonic_player_bp (cast `/Game/Roles/Designer/Owen/Bps/Twonic_Player_BP` OtherActor))
  (bind _returnvalue (`|SpawnActorFromClass` "/Game/Roles/Designer/Lewis/Effects/BP_Mana_Aura.BP_Mana_Aura_C" (`KismetMathLibrary.Conv_VectorToTransform` (`SceneComponent.K2_GetComponentLocation` (`Character.Mesh` _astwonic_player_bp))) "Undefined" "OverrideRootScale" null null))
  (set `self.ManaOn` true))

(fn `UserConstructionScript`)