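; Grid path puzzle where overlapping trigger tiles lights a route from a start core through cores A–Y to an end core.
; Each overlap uses Condition to compare the last lit tile, held in Current, against hardcoded neighbours; a match sets that tile's flag, turns it blue and replaces Current.
; Start appends without clearing, C follows only Start, and End only W.
; Tile O stores "0", so neighbour checks for "O" fail.
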(event `self.StartColl.OnComponentBeginOverlap`
  (params (OverlappedComponent :type "PrimitiveComponent Object Reference") (OtherActor :type "Actor Object Reference") (OtherComp :type "PrimitiveComponent Object Reference") (OtherBodyIndex :type Integer) (bFromSweep :type Boolean) (SweepResult :type "HitResult Structure (by ref)"))
  (set `self.CSTA` true)
  (`PrimitiveComponent.SetMaterial` (`self.CoreStart`) 0 "/Game/Roles/Designer/Clayton/Colours/Blue.Blue")
  (`KismetArrayLibrary.Array_Add` (`self.Current`) "ST"))

(event `self.AColl.OnComponentBeginOverlap`
  (params (OverlappedComponent :type "PrimitiveComponent Object Reference") (OtherActor :type "Actor Object Reference") (OtherComp :type "PrimitiveComponent Object Reference") (OtherBodyIndex :type Integer) (bFromSweep :type Boolean) (SweepResult :type "HitResult Structure (by ref)"))
  (bind (_check1 _check2) (`self.Condition` "B" "F"))
  (bind _current (`self.Current`))
  (if _check1
    (set `self.CAA` true :!label _label)
    (`PrimitiveComponent.SetMaterial` (`self.CoreA`) 0 "/Game/Roles/Designer/Clayton/Colours/Blue.Blue")
    (`KismetArrayLibrary.Array_Clear` _current)
    (`KismetArrayLibrary.Array_Add` _current "A")
    (elif _check2
      (goto _label))))

(event `self.BColl.OnComponentBeginOverlap`
  (params (OverlappedComponent :type "PrimitiveComponent Object Reference") (OtherActor :type "Actor Object Reference") (OtherComp :type "PrimitiveComponent Object Reference") (OtherBodyIndex :type Integer) (bFromSweep :type Boolean) (SweepResult :type "HitResult Structure (by ref)"))
  (bind (_check1 _check2 _check3) (`self.Condition` "A" "C" "G"))
  (bind _current (`self.Current`))
  (if _check1
    (set `self.CBA` true :!label _label_2)
    (`PrimitiveComponent.SetMaterial` (`self.CoreB`) 0 "/Game/Roles/Designer/Clayton/Colours/Blue.Blue")
    (`KismetArrayLibrary.Array_Clear` _current)
    (`KismetArrayLibrary.Array_Add` _current "B")
    (elif _check2
      (goto _label_2)
      (elif _check3
        (goto _label_2)))))

(event `self.CColl.OnComponentBeginOverlap`
  (params (OverlappedComponent :type "PrimitiveComponent Object Reference") (OtherActor :type "Actor Object Reference") (OtherComp :type "PrimitiveComponent Object Reference") (OtherBodyIndex :type Integer) (bFromSweep :type Boolean) (SweepResult :type "HitResult Structure (by ref)"))
  (bind _current (`self.Current`))
  (if (`self.Condition` "ST")
    (set `self.CCA` true)
    (`PrimitiveComponent.SetMaterial` (`self.CoreC`) 0 "/Game/Roles/Designer/Clayton/Colours/Blue.Blue")
    (`KismetArrayLibrary.Array_Clear` _current)
    (`KismetArrayLibrary.Array_Add` _current "C")))

(event `self.DColl.OnComponentBeginOverlap`
  (params (OverlappedComponent :type "PrimitiveComponent Object Reference") (OtherActor :type "Actor Object Reference") (OtherComp :type "PrimitiveComponent Object Reference") (OtherBodyIndex :type Integer) (bFromSweep :type Boolean) (SweepResult :type "HitResult Structure (by ref)"))
  (bind (_check1 _check2 _check3) (`self.Condition` "C" "E" "I"))
  (bind _current (`self.Current`))
  (if _check1
    (set `self.CDA` true :!label _label_3)
    (`PrimitiveComponent.SetMaterial` (`self.CoreD`) 0 "/Game/Roles/Designer/Clayton/Colours/Blue.Blue")
    (`KismetArrayLibrary.Array_Clear` _current)
    (`KismetArrayLibrary.Array_Add` _current "D")
    (elif _check2
      (goto _label_3)
      (elif _check3
        (goto _label_3)))))

(event `self.EColl.OnComponentBeginOverlap`
  (params (OverlappedComponent :type "PrimitiveComponent Object Reference") (OtherActor :type "Actor Object Reference") (OtherComp :type "PrimitiveComponent Object Reference") (OtherBodyIndex :type Integer) (bFromSweep :type Boolean) (SweepResult :type "HitResult Structure (by ref)"))
  (bind (_check1 _check2) (`self.Condition` "D" "J"))
  (bind _current (`self.Current`))
  (if _check1
    (set `self.CEA` true :!label _label_4)
    (`PrimitiveComponent.SetMaterial` (`self.CoreE`) 0 "/Game/Roles/Designer/Clayton/Colours/Blue.Blue")
    (`KismetArrayLibrary.Array_Clear` _current)
    (`KismetArrayLibrary.Array_Add` _current "E")
    (elif _check2
      (goto _label_4))))

(event `self.FColl.OnComponentBeginOverlap`
  (params (OverlappedComponent :type "PrimitiveComponent Object Reference") (OtherActor :type "Actor Object Reference") (OtherComp :type "PrimitiveComponent Object Reference") (OtherBodyIndex :type Integer) (bFromSweep :type Boolean) (SweepResult :type "HitResult Structure (by ref)"))
  (bind (_check1 _check2 _check3) (`self.Condition` "A" "G" "K"))
  (bind _current (`self.Current`))
  (if _check1
    (set `self.CFA` true :!label _label_5)
    (`PrimitiveComponent.SetMaterial` (`self.CoreF`) 0 "/Game/Roles/Designer/Clayton/Colours/Blue.Blue")
    (`KismetArrayLibrary.Array_Clear` _current)
    (`KismetArrayLibrary.Array_Add` _current "F")
    (elif _check2
      (goto _label_5)
      (elif _check3
        (goto _label_5)))))

(event `self.GColl.OnComponentBeginOverlap`
  (params (OverlappedComponent :type "PrimitiveComponent Object Reference") (OtherActor :type "Actor Object Reference") (OtherComp :type "PrimitiveComponent Object Reference") (OtherBodyIndex :type Integer) (bFromSweep :type Boolean) (SweepResult :type "HitResult Structure (by ref)"))
  (bind (_check1 _check2 _check3 _check4) (`self.Condition` "B" "F" "H" "L"))
  (bind _current (`self.Current`))
  (if _check1
    (set `self.CGA` true :!label _label_6)
    (`PrimitiveComponent.SetMaterial` (`self.CoreG`) 0 "/Game/Roles/Designer/Clayton/Colours/Blue.Blue")
    (`KismetArrayLibrary.Array_Clear` _current)
    (`KismetArrayLibrary.Array_Add` _current "G")
    (elif _check2
      (goto _label_6)
      (elif _check3
        (goto _label_6)
        (elif _check4
          (goto _label_6))))))

(event `self.HColl.OnComponentBeginOverlap`
  (params (OverlappedComponent :type "PrimitiveComponent Object Reference") (OtherActor :type "Actor Object Reference") (OtherComp :type "PrimitiveComponent Object Reference") (OtherBodyIndex :type Integer) (bFromSweep :type Boolean) (SweepResult :type "HitResult Structure (by ref)"))
  (bind (_check1 _check2 _check3 _check4) (`self.Condition` "C" "I" "M" "G"))
  (bind _current (`self.Current`))
  (if _check1
    (set `self.CHA` true :!label _label_7)
    (`PrimitiveComponent.SetMaterial` (`self.CoreH`) 0 "/Game/Roles/Designer/Clayton/Colours/Blue.Blue")
    (`KismetArrayLibrary.Array_Clear` _current)
    (`KismetArrayLibrary.Array_Add` _current "H")
    (elif _check2
      (goto _label_7)
      (elif _check3
        (goto _label_7)
        (elif _check4
          (goto _label_7))))))

(event `self.IColl.OnComponentBeginOverlap`
  (params (OverlappedComponent :type "PrimitiveComponent Object Reference") (OtherActor :type "Actor Object Reference") (OtherComp :type "PrimitiveComponent Object Reference") (OtherBodyIndex :type Integer) (bFromSweep :type Boolean) (SweepResult :type "HitResult Structure (by ref)"))
  (bind (_check1 _check2 _check3 _check4) (`self.Condition` "H" "D" "J" "N"))
  (bind _current (`self.Current`))
  (if _check1
    (set `self.CIA` true :!label _label_8)
    (`PrimitiveComponent.SetMaterial` (`self.CoreI`) 0 "/Game/Roles/Designer/Clayton/Colours/Blue.Blue")
    (`KismetArrayLibrary.Array_Clear` _current)
    (`KismetArrayLibrary.Array_Add` _current "I")
    (elif _check2
      (goto _label_8)
      (elif _check3
        (goto _label_8)
        (elif _check4
          (goto _label_8))))))

(event `self.JColl.OnComponentBeginOverlap`
  (params (OverlappedComponent :type "PrimitiveComponent Object Reference") (OtherActor :type "Actor Object Reference") (OtherComp :type "PrimitiveComponent Object Reference") (OtherBodyIndex :type Integer) (bFromSweep :type Boolean) (SweepResult :type "HitResult Structure (by ref)"))
  (bind (_check1 _check2 _check3 _check4) (`self.Condition` "E" "I" "O"))
  (bind _current (`self.Current`))
  (if _check1
    (set `self.CJA` true :!label _label_9)
    (`PrimitiveComponent.SetMaterial` (`self.CoreJ`) 0 "/Game/Roles/Designer/Clayton/Colours/Blue.Blue")
    (`KismetArrayLibrary.Array_Clear` _current)
    (`KismetArrayLibrary.Array_Add` _current "J")
    (elif _check2
      (goto _label_9)
      (elif _check3
        (goto _label_9)
        (elif _check4
          (goto _label_9))))))

(event `self.KColl.OnComponentBeginOverlap`
  (params (OverlappedComponent :type "PrimitiveComponent Object Reference") (OtherActor :type "Actor Object Reference") (OtherComp :type "PrimitiveComponent Object Reference") (OtherBodyIndex :type Integer) (bFromSweep :type Boolean) (SweepResult :type "HitResult Structure (by ref)"))
  (bind (_check1 _check2 _check3 _check4) (`self.Condition` "F" "L" "P"))
  (bind _current (`self.Current`))
  (if _check1
    (set `self.CKA` true :!label _label_10)
    (`PrimitiveComponent.SetMaterial` (`self.CoreK`) 0 "/Game/Roles/Designer/Clayton/Colours/Blue.Blue")
    (`KismetArrayLibrary.Array_Clear` _current)
    (`KismetArrayLibrary.Array_Add` _current "K")
    (elif _check2
      (goto _label_10)
      (elif _check3
        (goto _label_10)
        (elif _check4
          (goto _label_10))))))

(event `self.LColl.OnComponentBeginOverlap`
  (params (OverlappedComponent :type "PrimitiveComponent Object Reference") (OtherActor :type "Actor Object Reference") (OtherComp :type "PrimitiveComponent Object Reference") (OtherBodyIndex :type Integer) (bFromSweep :type Boolean) (SweepResult :type "HitResult Structure (by ref)"))
  (bind (_check1 _check2 _check3 _check4) (`self.Condition` "G" "M" "Q" "K"))
  (bind _current (`self.Current`))
  (if _check1
    (set `self.CLA` true :!label _label_11)
    (`PrimitiveComponent.SetMaterial` (`self.CoreL`) 0 "/Game/Roles/Designer/Clayton/Colours/Blue.Blue")
    (`KismetArrayLibrary.Array_Clear` _current)
    (`KismetArrayLibrary.Array_Add` _current "L")
    (elif _check2
      (goto _label_11)
      (elif _check3
        (goto _label_11)
        (elif _check4
          (goto _label_11))))))

(event `self.MColl.OnComponentBeginOverlap`
  (params (OverlappedComponent :type "PrimitiveComponent Object Reference") (OtherActor :type "Actor Object Reference") (OtherComp :type "PrimitiveComponent Object Reference") (OtherBodyIndex :type Integer) (bFromSweep :type Boolean) (SweepResult :type "HitResult Structure (by ref)"))
  (bind (_check1 _check2 _check3 _check4) (`self.Condition` "H" "N" "R" "L"))
  (bind _current (`self.Current`))
  (if _check1
    (set `self.CMA` true :!label _label_12)
    (`PrimitiveComponent.SetMaterial` (`self.CoreM`) 0 "/Game/Roles/Designer/Clayton/Colours/Blue.Blue")
    (`KismetArrayLibrary.Array_Clear` _current)
    (`KismetArrayLibrary.Array_Add` _current "M")
    (elif _check2
      (goto _label_12)
      (elif _check3
        (goto _label_12)
        (elif _check4
          (goto _label_12))))))

(event `self.NColl.OnComponentBeginOverlap`
  (params (OverlappedComponent :type "PrimitiveComponent Object Reference") (OtherActor :type "Actor Object Reference") (OtherComp :type "PrimitiveComponent Object Reference") (OtherBodyIndex :type Integer) (bFromSweep :type Boolean) (SweepResult :type "HitResult Structure (by ref)"))
  (bind (_check1 _check2 _check3 _check4) (`self.Condition` "I" "O" "S" "M"))
  (bind _current (`self.Current`))
  (if _check1
    (set `self.CNA` true :!label _label_13)
    (`PrimitiveComponent.SetMaterial` (`self.CoreN`) 0 "/Game/Roles/Designer/Clayton/Colours/Blue.Blue")
    (`KismetArrayLibrary.Array_Clear` _current)
    (`KismetArrayLibrary.Array_Add` _current "N")
    (elif _check2
      (goto _label_13)
      (elif _check3
        (goto _label_13)
        (elif _check4
          (goto _label_13))))))

(event `self.OColl.OnComponentBeginOverlap`
  (params (OverlappedComponent :type "PrimitiveComponent Object Reference") (OtherActor :type "Actor Object Reference") (OtherComp :type "PrimitiveComponent Object Reference") (OtherBodyIndex :type Integer) (bFromSweep :type Boolean) (SweepResult :type "HitResult Structure (by ref)"))
  (bind (_check1 _check2 _check3) (`self.Condition` "J" "T" "N"))
  (bind _current (`self.Current`))
  (if _check1
    (set `self.COA` true :!label _label_14)
    (`PrimitiveComponent.SetMaterial` (`self.CoreO`) 0 "/Game/Roles/Designer/Clayton/Colours/Blue.Blue")
    (`KismetArrayLibrary.Array_Clear` _current)
    (`KismetArrayLibrary.Array_Add` _current "0")
    (elif _check2
      (goto _label_14)
      (elif _check3
        (goto _label_14)))))

(event `self.PColl.OnComponentBeginOverlap`
  (params (OverlappedComponent :type "PrimitiveComponent Object Reference") (OtherActor :type "Actor Object Reference") (OtherComp :type "PrimitiveComponent Object Reference") (OtherBodyIndex :type Integer) (bFromSweep :type Boolean) (SweepResult :type "HitResult Structure (by ref)"))
  (bind (_check1 _check2 _check3) (`self.Condition` "K" "Q" "U"))
  (bind _current (`self.Current`))
  (if _check1
    (set `self.CPA` true :!label _label_15)
    (`PrimitiveComponent.SetMaterial` (`self.CoreP`) 0 "/Game/Roles/Designer/Clayton/Colours/Blue.Blue")
    (`KismetArrayLibrary.Array_Clear` _current)
    (`KismetArrayLibrary.Array_Add` _current "P")
    (elif _check2
      (goto _label_15)
      (elif _check3
        (goto _label_15)))))

(event `self.QColl.OnComponentBeginOverlap`
  (params (OverlappedComponent :type "PrimitiveComponent Object Reference") (OtherActor :type "Actor Object Reference") (OtherComp :type "PrimitiveComponent Object Reference") (OtherBodyIndex :type Integer) (bFromSweep :type Boolean) (SweepResult :type "HitResult Structure (by ref)"))
  (bind (_check1 _check2 _check3 _check4) (`self.Condition` "P" "L" "R" "V"))
  (bind _current (`self.Current`))
  (if _check1
    (set `self.CQA` true :!label _label_16)
    (`PrimitiveComponent.SetMaterial` (`self.CoreQ`) 0 "/Game/Roles/Designer/Clayton/Colours/Blue.Blue")
    (`KismetArrayLibrary.Array_Clear` _current)
    (`KismetArrayLibrary.Array_Add` _current "Q")
    (elif _check2
      (goto _label_16)
      (elif _check3
        (goto _label_16)
        (elif _check4
          (goto _label_16))))))

(event `self.RColl.OnComponentBeginOverlap`
  (params (OverlappedComponent :type "PrimitiveComponent Object Reference") (OtherActor :type "Actor Object Reference") (OtherComp :type "PrimitiveComponent Object Reference") (OtherBodyIndex :type Integer) (bFromSweep :type Boolean) (SweepResult :type "HitResult Structure (by ref)"))
  (bind (_check1 _check2 _check3 _check4) (`self.Condition` "Q" "M" "S" "W"))
  (bind _current (`self.Current`))
  (if _check1
    (set `self.CRA` true :!label _label_17)
    (`PrimitiveComponent.SetMaterial` (`self.CoreR`) 0 "/Game/Roles/Designer/Clayton/Colours/Blue.Blue")
    (`KismetArrayLibrary.Array_Clear` _current)
    (`KismetArrayLibrary.Array_Add` _current "R")
    (elif _check2
      (goto _label_17)
      (elif _check3
        (goto _label_17)
        (elif _check4
          (goto _label_17))))))

(event `self.SColl.OnComponentBeginOverlap`
  (params (OverlappedComponent :type "PrimitiveComponent Object Reference") (OtherActor :type "Actor Object Reference") (OtherComp :type "PrimitiveComponent Object Reference") (OtherBodyIndex :type Integer) (bFromSweep :type Boolean) (SweepResult :type "HitResult Structure (by ref)"))
  (bind (_check1 _check2 _check3 _check4) (`self.Condition` "R" "N" "T" "X"))
  (bind _current (`self.Current`))
  (if _check1
    (set `self.CSA` true :!label _label_18)
    (`PrimitiveComponent.SetMaterial` (`self.coreS`) 0 "/Game/Roles/Designer/Clayton/Colours/Blue.Blue")
    (`KismetArrayLibrary.Array_Clear` _current)
    (`KismetArrayLibrary.Array_Add` _current "S")
    (elif _check2
      (goto _label_18)
      (elif _check3
        (goto _label_18)
        (elif _check4
          (goto _label_18))))))

(event `self.TColl.OnComponentBeginOverlap`
  (params (OverlappedComponent :type "PrimitiveComponent Object Reference") (OtherActor :type "Actor Object Reference") (OtherComp :type "PrimitiveComponent Object Reference") (OtherBodyIndex :type Integer) (bFromSweep :type Boolean) (SweepResult :type "HitResult Structure (by ref)"))
  (bind (_check1 _check2 _check3) (`self.Condition` "S" "O" "Y"))
  (bind _current (`self.Current`))
  (if _check1
    (set `self.CTA` true :!label _label_19)
    (`PrimitiveComponent.SetMaterial` (`self.CoreT`) 0 "/Game/Roles/Designer/Clayton/Colours/Blue.Blue")
    (`KismetArrayLibrary.Array_Clear` _current)
    (`KismetArrayLibrary.Array_Add` _current "T")
    (elif _check2
      (goto _label_19)
      (elif _check3
        (goto _label_19)))))

(event `self.UColl.OnComponentBeginOverlap`
  (params (OverlappedComponent :type "PrimitiveComponent Object Reference") (OtherActor :type "Actor Object Reference") (OtherComp :type "PrimitiveComponent Object Reference") (OtherBodyIndex :type Integer) (bFromSweep :type Boolean) (SweepResult :type "HitResult Structure (by ref)"))
  (bind (_check1 _check2) (`self.Condition` "P" "V"))
  (bind _current (`self.Current`))
  (if _check1
    (set `self.CUA` true :!label _label_20)
    (`PrimitiveComponent.SetMaterial` (`self.CoreU`) 0 "/Game/Roles/Designer/Clayton/Colours/Blue.Blue")
    (`KismetArrayLibrary.Array_Clear` _current)
    (`KismetArrayLibrary.Array_Add` _current "U")
    (elif _check2
      (goto _label_20))))

(event `self.VColl.OnComponentBeginOverlap`
  (params (OverlappedComponent :type "PrimitiveComponent Object Reference") (OtherActor :type "Actor Object Reference") (OtherComp :type "PrimitiveComponent Object Reference") (OtherBodyIndex :type Integer) (bFromSweep :type Boolean) (SweepResult :type "HitResult Structure (by ref)"))
  (bind (_check1 _check2 _check3) (`self.Condition` "U" "Q" "W"))
  (bind _current (`self.Current`))
  (if _check1
    (set `self.CVA` true :!label _label_21)
    (`PrimitiveComponent.SetMaterial` (`self.CoreV`) 0 "/Game/Roles/Designer/Clayton/Colours/Blue.Blue")
    (`KismetArrayLibrary.Array_Clear` _current)
    (`KismetArrayLibrary.Array_Add` _current "V")
    (elif _check2
      (goto _label_21)
      (elif _check3
        (goto _label_21)))))

(event `self.WColl.OnComponentBeginOverlap`
  (params (OverlappedComponent :type "PrimitiveComponent Object Reference") (OtherActor :type "Actor Object Reference") (OtherComp :type "PrimitiveComponent Object Reference") (OtherBodyIndex :type Integer) (bFromSweep :type Boolean) (SweepResult :type "HitResult Structure (by ref)"))
  (bind (_check1 _check2 _check3) (`self.Condition` "V" "R" "X"))
  (bind _current (`self.Current`))
  (if _check1
    (set `self.CWA` true :!label _label_22)
    (`PrimitiveComponent.SetMaterial` (`self.CoreW`) 0 "/Game/Roles/Designer/Clayton/Colours/Blue.Blue")
    (`KismetArrayLibrary.Array_Clear` _current)
    (`KismetArrayLibrary.Array_Add` _current "W")
    (elif _check2
      (goto _label_22)
      (elif _check3
        (goto _label_22)))))

(event `self.XColl.OnComponentBeginOverlap`
  (params (OverlappedComponent :type "PrimitiveComponent Object Reference") (OtherActor :type "Actor Object Reference") (OtherComp :type "PrimitiveComponent Object Reference") (OtherBodyIndex :type Integer) (bFromSweep :type Boolean) (SweepResult :type "HitResult Structure (by ref)"))
  (bind (_check1 _check2 _check3) (`self.Condition` "W" "S" "Y"))
  (bind _current (`self.Current`))
  (if _check1
    (set `self.CXA` true :!label _label_23)
    (`PrimitiveComponent.SetMaterial` (`self.CoreX`) 0 "/Game/Roles/Designer/Clayton/Colours/Blue.Blue")
    (`KismetArrayLibrary.Array_Clear` _current)
    (`KismetArrayLibrary.Array_Add` _current "X")
    (elif _check2
      (goto _label_23)
      (elif _check3
        (goto _label_23)))))

(event `self.YColl.OnComponentBeginOverlap`
  (params (OverlappedComponent :type "PrimitiveComponent Object Reference") (OtherActor :type "Actor Object Reference") (OtherComp :type "PrimitiveComponent Object Reference") (OtherBodyIndex :type Integer) (bFromSweep :type Boolean) (SweepResult :type "HitResult Structure (by ref)"))
  (bind (_check1 _check2) (`self.Condition` "X" "T"))
  (bind _current (`self.Current`))
  (if _check1
    (set `self.CYA` true :!label _label_24)
    (`PrimitiveComponent.SetMaterial` (`self.CoreY`) 0 "/Game/Roles/Designer/Clayton/Colours/Blue.Blue")
    (`KismetArrayLibrary.Array_Clear` _current)
    (`KismetArrayLibrary.Array_Add` _current "Y")
    (elif _check2
      (goto _label_24))))

(event `self.EndColl.OnComponentBeginOverlap`
  (params (OverlappedComponent :type "PrimitiveComponent Object Reference") (OtherActor :type "Actor Object Reference") (OtherComp :type "PrimitiveComponent Object Reference") (OtherBodyIndex :type Integer) (bFromSweep :type Boolean) (SweepResult :type "HitResult Structure (by ref)"))
  (if (`self.Condition` "W")
    (set `self.CENDA` true)
    (`PrimitiveComponent.SetMaterial` (`self.Coreend`) 0 "/Game/Roles/Designer/Clayton/Colours/Blue.Blue")
    (`KismetArrayLibrary.Array_Clear` (`self.Current`))))

(fn `UserConstructionScript`)