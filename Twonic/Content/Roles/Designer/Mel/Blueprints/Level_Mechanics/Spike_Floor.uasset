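; Spike floor trap that springs when the Twonic player overlaps its trigger box.
; An activate timeline moves the spikes along Z, then after a short delay a retract timeline moves them back.
; An activation flag ignores further overlaps until retraction finishes.
; The Blueprint only handles movement and contains no damage logic.
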(event `self.Trigger_Box.OnComponentBeginOverlap`
  (params (OverlappedComponent :type "PrimitiveComponent Object Reference") (OtherActor :type "Actor Object Reference") (OtherComp :type "PrimitiveComponent Object Reference") (OtherBodyIndex :type Integer) (bFromSweep :type Boolean) (SweepResult :type "HitResult Structure (by ref)"))
  (cast `/Game/Roles/Designer/Owen/Bps/Twonic_Player_BP` OtherActor)
  (if (not (`self.Spikes_Activated`))
    (set `self.Spikes_Activated` true)
    (bind (_direction _spikes_activate) (`Timeline|Spikes_Activate` :!via `PlayFromStart`)
      (:`Update`
        (`SceneComponent.K2_SetRelativeLocation` (`self.Spikes`) (`KismetMathLibrary.MakeVector` 0.0 0.0 _spikes_activate) false false))
      (:`Finished`
        (`KismetSystemLibrary.Delay` 0.5)
        (bind (_direction_2 _spikes_retract) (`Timeline|Spikes_Retract` :!via `PlayFromStart`)
          (:`Update`
            (`SceneComponent.K2_SetRelativeLocation` (`self.Spikes`) (`KismetMathLibrary.MakeVector` 0.0 0.0 _spikes_retract) false false))
          (:`Finished`
            (set `self.Spikes_Activated` false)))))))

(fn `UserConstructionScript`)