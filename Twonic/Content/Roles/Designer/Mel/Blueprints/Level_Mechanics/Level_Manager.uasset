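; Level manager Blueprint that tracks statue puzzle progress and records the player's respawn location.
; On BeginPlay it casts the player pawn to Twonic_Player_BP and stores its starting position as PlayerRespawnLoc, which this Blueprint does not itself use.
; StatueActivated increments a counter and opens StatuePuzzleGate once the count reaches StatuesNeeded.
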(event `self.ReceiveBeginPlay`
  (bind _astwonic_player_bp (cast `/Game/Roles/Designer/Owen/Bps/Twonic_Player_BP` (`GameplayStatics.GetPlayerPawn` 0)))
  (set `self.Player_Respawn_Loc` (`self.K2_GetActorLocation` _astwonic_player_bp)))

(fn `Statue_Activated`
  (set `self.Statues_Activated` (+ (`self.Statues_Activated`) 1))
  (if (>= (`self.Statues_Activated`) (`self.Statues_Needed`))
    (`/Game/Roles/Designer/Mel/Blueprints/Level_Mechanics/BP_Openable_Gate.Open_Gate` (`self.Statue_Puzzle_Gate`))))

(fn `UserConstructionScript`)