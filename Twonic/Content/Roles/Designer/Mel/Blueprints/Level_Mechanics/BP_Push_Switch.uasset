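; BP_Push_Switch is an interactable switch that triggers a linked bridge drop or gate opening in a level.
; An activation range volume enables input when Twonic_Player_BP enters and disables it when an overlap ends.
; On Interact, it calls DropBridge or, failing that flag, OpenGate, based on its ActivatesBridge and ActivatesGate booleans.
; It then destroys the activation range, making the switch single-use.
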(event `self.Activation_Range.OnComponentBeginOverlap`
  (params (OverlappedComponent :type "PrimitiveComponent Object Reference") (OtherActor :type "Actor Object Reference") (OtherComp :type "PrimitiveComponent Object Reference") (OtherBodyIndex :type Integer) (bFromSweep :type Boolean) (SweepResult :type "HitResult Structure (by ref)"))
  (cast `/Game/Roles/Designer/Owen/Bps/Twonic_Player_BP` OtherActor)
  (`self.EnableInput` (`GameplayStatics.GetPlayerController` 0)))

(event `self.Activation_Range.OnComponentEndOverlap`
  (params (OverlappedComponent :type "PrimitiveComponent Object Reference") (OtherActor :type "Actor Object Reference") (OtherComp :type "PrimitiveComponent Object Reference") (OtherBodyIndex :type Integer))
  (`self.DisableInput` (`GameplayStatics.GetPlayerController` 0)))

(event `InputAction|Interact`
  (params (Key :type "Key Structure"))
  (:`Pressed`
    (if (`self.Activates_Bridge`)
      (`/Game/Roles/Designer/Mel/Blueprints/Level_Mechanics/BP_Droppable_Bridge.Drop_Bridge` (`self.Bridge`))
      (`ActorComponent.K2_DestroyComponent` (`self.Activation_Range`))
      (elif (`self.Activates_Gate`)
        (`/Game/Roles/Designer/Mel/Blueprints/Level_Mechanics/BP_Openable_Gate.Open_Gate` (`self.Gate`))
        (`ActorComponent.K2_DestroyComponent` (`self.Activation_Range`))))))

(fn `UserConstructionScript`)