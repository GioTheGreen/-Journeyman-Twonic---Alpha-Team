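; Floor spike trap that raises and retracts spikes and damages Twonic_Player_BP on hitbox overlap.
; With IsAutomatic set, a looping timer started at BeginPlay runs the raise, pause and retract cycle.
; The player entering the trigger box also fires it after a short delay, with SpikesActivated blocking re-triggers until retraction ends.
; Separate timelines for each mode drive the Spikes' relative Z location.
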(event `self.ReceiveBeginPlay`
  ;[1 1 1] Automatic: If variable is checked then spikes automatically activate and deactivate on a timer.
  (if (`self.Is_Automatic`)
    (`KismetSystemLibrary.K2_SetTimerDelegate` (delegate `Auto_Trap`) 10.5 true)
    (`self.Auto_Trap`)))

(event `Auto_Trap`
  ;[1 1 1] Automatic: If variable is checked then spikes automatically activate and deactivate on a timer.
  (bind (_direction _spikes_activate) (`Timeline|Auto_Activate` :!via `PlayFromStart`)
    (:`Update`
      (`SceneComponent.K2_SetRelativeLocation` (`self.Spikes`) (`KismetMathLibrary.MakeVector` 0.0 0.0 _spikes_activate) false false))
    (:`Finished`
      (`KismetSystemLibrary.Delay` 0.5)
      (bind (_direction_2 _spikes_retract) (`Timeline|Auto_Retract` :!via `PlayFromStart`)
        (:`Update`
          (`SceneComponent.K2_SetRelativeLocation` (`self.Spikes`) (`KismetMathLibrary.MakeVector` 0.0 0.0 _spikes_retract) false false))))))

(event `self.Trigger_Box.OnComponentBeginOverlap`
  (params (OverlappedComponent :type "PrimitiveComponent Object Reference") (OtherActor :type "Actor Object Reference") (OtherComp :type "PrimitiveComponent Object Reference") (OtherBodyIndex :type Integer) (bFromSweep :type Boolean) (SweepResult :type "HitResult Structure (by ref)"))
  ;[1 1 1] Player Activated: When player steps on spikes after a short delay spikes activate and then retract. Cannot be reactivated while spikes are still retracting.
  (cast `/Game/Roles/Designer/Owen/Bps/Twonic_Player_BP` OtherActor)
  (if (not (`self.Spikes_Activated`))
    (`KismetSystemLibrary.Delay` 0.5)
    (set `self.Spikes_Activated` true)
    (bind (_direction _spikes_activate) (`Timeline|Spikes_Activate` :!via `PlayFromStart`)
      (:`Update`
        (`SceneComponent.K2_SetRelativeLocation` (`self.Spikes`) (`KismetMathLibrary.MakeVector` 0.0 0.0 _spikes_activate) false false))
      (:`Finished`
        (`KismetSystemLibrary.Delay` 0.5)
        (bind (_direction_2 _spikes_retract) (`Timeline|Spikes_Retract` :!via `PlayFromStart`)
          (:`Update`
            (`SceneComponent.K2_SetRelativeLocation` (`self.Spikes`) (`KismetMathLibrary.MakeVector` 0.0 0.0 _spikes_retract) false false))
          (:`Finished`
            (set `self.Spikes_Activated` false)))))))

(event `self.Hitbox.OnComponentBeginOverlap`
  (params (OverlappedComponent :type "PrimitiveComponent Object Reference") (OtherActor :type "Actor Object Reference") (OtherComp :type "PrimitiveComponent Object Reference") (OtherBodyIndex :type Integer) (bFromSweep :type Boolean) (SweepResult :type "HitResult Structure (by ref)"))
  ;[1 1 1] Player Activated: When player steps on spikes after a short delay spikes activate and then retract. Cannot be reactivated while spikes are still retracting.
  (bind _astwonic_player_bp (cast `/Game/Roles/Designer/Owen/Bps/Twonic_Player_BP` OtherActor))
  (`GameplayStatics.ApplyDamage` _astwonic_player_bp 25.0 null null "/Script/Engine.DamageType"))

(fn `UserConstructionScript`)