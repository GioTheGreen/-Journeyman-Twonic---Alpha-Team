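; Wishing well level actor that takes one Money from the player each time Interact is pressed nearby, with no reward given in this Blueprint.
; Entering the activation range as the player caches the character and enables input on the well; any overlap ending disables it.
; Interact checks for a positive Money balance, then rebuilds the player's LevellingStructure with Money reduced and all other fields copied unchanged.
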(event `self.Activation_Range.OnComponentBeginOverlap`
  (params (OverlappedComponent :type "PrimitiveComponent Object Reference") (OtherActor :type "Actor Object Reference") (OtherComp :type "PrimitiveComponent Object Reference") (OtherBodyIndex :type Integer) (bFromSweep :type Boolean) (SweepResult :type "HitResult Structure (by ref)"))
  (bind _astwonic_player_bp (cast `/Game/Roles/Designer/Owen/Bps/Twonic_Player_BP` OtherActor))
  (`self.EnableInput` (`GameplayStatics.GetPlayerController` 0)))

(event `self.Activation_Range.OnComponentEndOverlap`
  (params (OverlappedComponent :type "PrimitiveComponent Object Reference") (OtherActor :type "Actor Object Reference") (OtherComp :type "PrimitiveComponent Object Reference") (OtherBodyIndex :type Integer))
  (`self.DisableInput` (`GameplayStatics.GetPlayerController` 0)))

(event `InputAction|Interact`
  (params (Key :type "Key Structure"))
  (:`Pressed`
    (bind (_levellingstructure_attackcurrency _levellingstructure_defensecurrency _levellingstructure_healthcurrency _levellingstructure_potioncurrency _levellingstructure_staminacurrency _levellingstructure_manacurrency _levellingstructure_money _levellingstructure_attlvl _levellingstructure_deflvl _levellingstructure_hplvl _levellingstructure_potlvl _levellingstructure_stalvl _levellingstructure_mplvl) (break `/Game/Roles/Designer/Michael/LevelUp/LevelStats` (`/Game/Roles/Designer/Owen/Bps/Twonic_Player_BP.LevellingStructure` (stale `self.Activation_Range.OnComponentBeginOverlap` _astwonic_player_bp))))
    (if (> _levellingstructure_money 0)
      (set `/Game/Roles/Designer/Owen/Bps/Twonic_Player_BP.LevellingStructure` (make `/Game/Roles/Designer/Michael/LevelUp/LevelStats` _levellingstructure_attackcurrency _levellingstructure_defensecurrency _levellingstructure_healthcurrency _levellingstructure_potioncurrency _levellingstructure_staminacurrency _levellingstructure_manacurrency (- _levellingstructure_money 1) _levellingstructure_attlvl _levellingstructure_deflvl _levellingstructure_hplvl _levellingstructure_potlvl _levellingstructure_stalvl _levellingstructure_mplvl) (stale `self.Activation_Range.OnComponentBeginOverlap` _astwonic_player_bp)))))

(fn `UserConstructionScript`)