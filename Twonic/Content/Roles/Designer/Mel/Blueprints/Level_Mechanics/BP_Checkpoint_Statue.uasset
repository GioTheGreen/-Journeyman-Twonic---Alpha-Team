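; BP_Checkpoint_Statue is a checkpoint statue the player interacts with to rest and set a respawn point.
; Entering the trigger area as Twonic_Player_BP enables the actor's input, and any actor leaving it disables that input.
; Pressing Interact refills the player's flasks and health to max and saves the statue's Scene location, cached at BeginPlay, as the LevelManager's respawn location.
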(event `self.ReceiveBeginPlay`
  (set `self.Spawn_Loc` (`SceneComponent.K2_GetComponentLocation` (`self.Scene`))))

(event `self.Trigger_Area.OnComponentBeginOverlap`
  (params (OverlappedComponent :type "PrimitiveComponent Object Reference") (OtherActor :type "Actor Object Reference") (OtherComp :type "PrimitiveComponent Object Reference") (OtherBodyIndex :type Integer) (bFromSweep :type Boolean) (SweepResult :type "HitResult Structure (by ref)"))
  (bind _astwonic_player_bp (cast `/Game/Roles/Designer/Owen/Bps/Twonic_Player_BP` OtherActor))
  (`self.EnableInput` (`GameplayStatics.GetPlayerController` 0)))

(event `self.Trigger_Area.OnComponentEndOverlap`
  (params (OverlappedComponent :type "PrimitiveComponent Object Reference") (OtherActor :type "Actor Object Reference") (OtherComp :type "PrimitiveComponent Object Reference") (OtherBodyIndex :type Integer))
  (`self.DisableInput` (`GameplayStatics.GetPlayerController` 0)))

(event `InputAction|Interact`
  (params (Key :type "Key Structure"))
  (:`Pressed`
    (set `/Game/Roles/Designer/Owen/Bps/Twonic_Player_BP.Current Flasks` (`/Game/Roles/Designer/Owen/Bps/Twonic_Player_BP.Max Flasks` (stale `self.Trigger_Area.OnComponentBeginOverlap` _astwonic_player_bp)) (stale `self.Trigger_Area.OnComponentBeginOverlap` _astwonic_player_bp))
    (set `/Game/Roles/Designer/Owen/Bps/Twonic_Player_BP.Current Health` (`/Game/Roles/Designer/Owen/Bps/Twonic_Player_BP.Max Health` (stale `self.Trigger_Area.OnComponentBeginOverlap` _astwonic_player_bp)) (stale `self.Trigger_Area.OnComponentBeginOverlap` _astwonic_player_bp))
    (set `/Game/Roles/Designer/Mel/Blueprints/Level_Mechanics/Level_Manager.Player_Respawn_Loc` (`self.Spawn_Loc`) (`self.Level_Manager`))))

(fn `UserConstructionScript`)