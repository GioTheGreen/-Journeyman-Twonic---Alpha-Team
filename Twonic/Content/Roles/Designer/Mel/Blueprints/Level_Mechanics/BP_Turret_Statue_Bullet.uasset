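; Statue turret that fires projectiles at the player when its pawn sensing component spots them.
; If Rotates is set, it first snaps to a look-at rotation using only roll and pitch, leaving yaw unwired.
; Firing spawns BP_Turret_Statue_Projectile at BulletSpawnLoc after a short wind-up, then holds a cooldown, with a Firing flag blocking overlapping shots.
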(event `self.LOS.OnSeePawn`
  (params (Pawn :type "Pawn Object Reference"))
  (bind _astwonic_player_bp (cast `/Game/Roles/Designer/Owen/Bps/Twonic_Player_BP` Pawn))
  (if (`self.Rotates?`)
    (`self.Face_Player`)
    (else
      (`self.Fire_Projectile`))))

(event `Fire_Projectile`
  (if (not (`self.Firing`))
    (set `self.Firing` true)
    (`KismetSystemLibrary.Delay` 0.5)
    (`|SpawnActorFromClass` "/Game/Roles/Designer/Mel/Blueprints/Level_Mechanics/BP_Turret_Statue_Projectile.BP_Turret_Statue_Projectile_C" (`SceneComponent.K2_GetComponentToWorld` (`self.Bullet_Spawn_Loc`)) "AlwaysSpawn" "OverrideRootScale" null null)
    (`KismetSystemLibrary.Delay` 2.0)
    (set `self.Firing` false)))

(event `Face_Player`
  (bind (_returnvalue_roll _returnvalue_pitch) (`KismetMathLibrary.BreakRotator` (`KismetMathLibrary.FindLookAtRotation` (`self.K2_GetActorLocation`) (`self.K2_GetActorLocation` (stale `self.LOS.OnSeePawn` _astwonic_player_bp)))))
  (`self.K2_SetActorRotation` (`KismetMathLibrary.MakeRotator` _returnvalue_roll _returnvalue_pitch))
  (`self.Fire_Projectile`))

(fn `UserConstructionScript`)