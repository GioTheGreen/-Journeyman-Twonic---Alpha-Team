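; Prayer obelisk puzzle piece that activates when the player prays continuously inside its trigger area for about two seconds.
; Entering the area starts a looping timer that polls the player's IsPraying flag and builds a counter, which resets on stopping or leaving.
; At the threshold it clears the timer, destroys the trigger, notifies the LevelManager through StatueActivated and lowers the obelisk with a timeline.
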(event `self.Trigger_Area.OnComponentBeginOverlap`
  (params (OverlappedComponent :type "PrimitiveComponent Object Reference") (OtherActor :type "Actor Object Reference") (OtherComp :type "PrimitiveComponent Object Reference") (OtherBodyIndex :type Integer) (bFromSweep :type Boolean) (SweepResult :type "HitResult Structure (by ref)"))
  (bind _astwonic_player_bp (cast `/Game/Roles/Designer/Owen/Bps/Twonic_Player_BP` OtherActor))
  (`KismetSystemLibrary.PrintString` "In Area")
  (bind _returnvalue (`KismetSystemLibrary.K2_SetTimerDelegate` (delegate `Recieving Prayer`) 0.2 true))
  (set `self.Prayer_Check` _returnvalue))

(event `Recieving Prayer`
  (if (`/Game/Roles/Designer/Owen/Bps/Twonic_Player_BP.Is_Praying` (stale `self.Trigger_Area.OnComponentBeginOverlap` _astwonic_player_bp))
    (`KismetSystemLibrary.PrintString` "Prayer Recieved")
    (set `self.Prayer_Time` (+ (`self.Prayer_Time`) 1.0))
    (if (== (`self.Prayer_Time`) 10.0)
      (`KismetSystemLibrary.K2_ClearAndInvalidateTimerHandle` (`self.Prayer_Check`))
      (`ActorComponent.K2_DestroyComponent` (`self.Trigger_Area`))
      (`KismetSystemLibrary.PrintString` "Activated")
      (`/Game/Roles/Designer/Mel/Blueprints/Level_Mechanics/Level_Manager.Statue_Activated` (`self.Level_Manager`))
      (bind (_direction _gate_move) (`Timeline|Lower Obelisk` :!via `PlayFromStart`)
        (:`Update`
          (`SceneComponent.K2_SetRelativeLocation` (`self.Obelisk`) (`KismetMathLibrary.MakeVector` 0.0 0.0 _gate_move) false false))))
    (else
      (`KismetSystemLibrary.PrintString` "No Prayer")
      (set `self.Prayer_Time` 0.0))))

(event `self.Trigger_Area.OnComponentEndOverlap`
  (params (OverlappedComponent :type "PrimitiveComponent Object Reference") (OtherActor :type "Actor Object Reference") (OtherComp :type "PrimitiveComponent Object Reference") (OtherBodyIndex :type Integer))
  (cast `/Game/Roles/Designer/Owen/Bps/Twonic_Player_BP` OtherActor)
  (`KismetSystemLibrary.K2_ClearAndInvalidateTimerHandle` (`self.Prayer_Check`))
  (set `self.Prayer_Time` 0.0))

(fn `UserConstructionScript`)